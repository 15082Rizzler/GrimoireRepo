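; Week2Character is a test player character Blueprint with basic walk, look and jump controls.
; On BeginPlay it adds the IMC_MyController Enhanced Input mapping context to the first player controller's local player subsystem.
; IA_Movement drives movement along the actor's forward and right vectors, and IA_LookAround feeds controller yaw and inverted pitch.
; Jump runs on a separate JumpAction input, starting on press and stopping on release.
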(event Input|EnhancedActionEvents|EnhancedInputActionIA_Movement
  (params (ActionValue :type Vector%202D%20Structure) (ElapsedSeconds :type Float%20%28double-precision%29) (TriggeredSeconds :type Float%20%28double-precision%29) (InputAction :type Input%20Action%20Object%20Reference :default "/Game/TestMapStuff/Core/IA_Movement.IA_Movement"))
  ;[0.04205 0.05172 0.15 0.5] WASD Movement System
  (Pawn|Input|AddMovementInput (Transformation|GetActorForwardVector) (.x ActionValue) false) ; Movement Up and Down
  (Pawn|Input|AddMovementInput (Transformation|GetActorRightVector) (.y ActionValue) false) ; Movement Left and Right
)

(event Input|EnhancedActionEvents|EnhancedInputActionIA_LookAround
  (params (ActionValue :type Vector%202D%20Structure) (ElapsedSeconds :type Float%20%28double-precision%29) (TriggeredSeconds :type Float%20%28double-precision%29) (InputAction :type Input%20Action%20Object%20Reference :default "/Game/TestMapStuff/Core/IA_LookAround.IA_LookAround"))
  ;[0.02375 0.03731 0.15 0.5] Look Around With Mouse
  (Pawn|Input|AddControllerYawInput (.x ActionValue))
  (Pawn|Input|AddControllerPitchInput (* (.y ActionValue) -1.0)))

(event EventBeginPlay
  ;[0.15 0.03828 0.03828 0.5] Controller Setup
  (Input|AddMappingContext (PlayerController|LocalPlayerSubsystems|GetEnhancedInputLocalPlayerSubsystem (Game|GetPlayerController 0)) "/Game/TestMapStuff/Core/IMC_MyController.IMC_MyController" 0 "(bIgnoreAllPressedKeysUntilRelease=True,bForceImmediately=False,bNotifyUserSettings=False)"))

(event Input|ActionEvents|InputActionJumpAction
  (params (Key :type Key%20Structure))
  (:Pressed
    (Character|Jump))
  (:Released
    (Character|StopJumping)))

(fn ConstructionScript)