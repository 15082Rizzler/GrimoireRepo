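; BP_Door2 is a double door the player opens by pressing E while standing in its trigger box.
; Overlap by a Week2Character enables input on the actor, and E plays the DoorOpening timeline, which yaws the left and right pivots.
; Leaving the box disables input, then reverses the timeline after a short delay to close the door.
; The text visibility and 2D sound nodes are unconnected and never run.
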(event OnComponentBeginOverlap(BoxCollision)
  (params (OverlappedComponent :type Primitive%20Component%20Object%20Reference) (OtherActor :type Actor%20Object%20Reference) (OtherComp :type Primitive%20Component%20Object%20Reference) (OtherBodyIndex :type Integer) (bFromSweep :type Boolean) (SweepResult :type Hit%20Result%20Structure%20%28by%20ref%29))
  ;[0.15 0.15 0.15 0.5] Enter the Trigger Zone
  (Utilities|Casting|CastToWeek2Character OtherActor)
  (Input|EnableInput (Game|GetPlayerController 0)))

(event OnComponentEndOverlap(BoxCollision)
  (params (OverlappedComponent :type Primitive%20Component%20Object%20Reference) (OtherActor :type Actor%20Object%20Reference) (OtherComp :type Primitive%20Component%20Object%20Reference) (OtherBodyIndex :type Integer))
  ;[0.15 0.15 0.15 0.5] Leaving The Trigger Zone
  (Utilities|Casting|CastToWeek2Character OtherActor)
  (Input|DisableInput (Game|GetPlayerController 0))
  ;[0.15 0.15 0.15 0.5] Press E to Open the Door
  (Utilities|FlowControl|Delay 1.0)
  (bind (_direction _leftdoor _rightdoor) (Timeline|DoorOpening Reverse)
    (:Update
      (Utilities|FlowControl|Sequence
        (:then_0
          (Transformation|SetRelativeRotation (Variables|Default|GetLeftPivot) (Math|Rotator|MakeRotator 0.0 0.0 _leftdoor) false false))
        (:then_1
          (Transformation|SetRelativeRotation (Variables|Default|GetRightPivot) (Math|Rotator|MakeRotator 0.0 0.0 _rightdoor) false false))))))

(event Input|KeyboardEvents|E
  (params (Key :type Key%20Structure))
  ;[0.15 0.15 0.15 0.5] Press E to Open the Door
  (:Pressed
    (bind (_direction _leftdoor _rightdoor) (Timeline|DoorOpening Play)
      (:Update
        (Utilities|FlowControl|Sequence
          (:then_0
            (Transformation|SetRelativeRotation (Variables|Default|GetLeftPivot) (Math|Rotator|MakeRotator 0.0 0.0 _leftdoor) false false))
          (:then_1
            (Transformation|SetRelativeRotation (Variables|Default|GetRightPivot) (Math|Rotator|MakeRotator 0.0 0.0 _rightdoor) false false)))))))

(fn ConstructionScript)