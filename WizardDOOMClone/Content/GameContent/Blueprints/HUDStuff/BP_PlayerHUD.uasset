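; Player HUD Blueprint that creates the main HUD widget, adds it to the viewport and acts as its access point.
; BeginPlay caches the widget and player 0's controlled BP_PlayerCharacter, which a separate SetupPlayerRef event later hands to the widget.
; Its other events are thin pass-throughs to the widget for adding key and primary or secondary spell icons, clearing spell icons and triggering text notifications.
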(event Custom|HUD_AddKeyIcon
  (params (Class :type User%20Widget%20Class%20Reference))
  (Default|AddKeyIcon (Variables|Default|GetWidgetREF) Class))

(event Custom|SetupPlayerRef
  (Default|SetPlayerRef (Variables|Default|GetWidgetREF) (Variables|Default|GetPlayerREF)))

(event Custom|HUD_AddPrimarySpellIcon
  (params (Class :type User%20Widget%20Class%20Reference))
  (Default|AddPrimarySpellIcon (Variables|Default|GetWidgetREF) Class))

(event Custom|HUD_AddSecondarySpellIcon
  (params (Class :type User%20Widget%20Class%20Reference))
  (Default|AddSecondarySpellIcon (Variables|Default|GetWidgetREF) Class))

(event Custom|HUD_TriggerNotification
  (params (InputText :type Text))
  (Default|TriggerNotification (Variables|Default|GetWidgetREF) InputText))

(event Custom|HUD_DestroySpellIcons
  (Default|DestroySpellIcons (Variables|Default|GetWidgetREF)))

(event EventBeginPlay
  (bind _returnvalue (Game|GetPlayerController 0))
  (bind _returnvalue_2 (UserInterface|CreateWidget "/Game/GameContent/Blueprints/HUDStuff/WB_MainPlayerHUD.WB_MainPlayerHUD_C" _returnvalue))
  (bind _output_get (Variables|Default|SetWidgetREF _returnvalue_2))
  (UserInterface|Viewport|AddtoViewport _output_get 0)
  (bind _asbp_player_character (Utilities|Casting|CastToBP_PlayerCharacter (Pawn|GetControlledPawn _returnvalue)))
  (Variables|Default|SetPlayerREF _asbp_player_character))

(fn ConstructionScript)