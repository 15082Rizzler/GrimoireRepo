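; Base enemy Blueprint with health, AI movement and a temporary freeze effect.
; Damage reduces health; on death it decrements the BP_EnemyManager's remaining count, has it clear doors when none remain, then destroys itself.
; Freeze sets an overlay material on root child static meshes, flags the AI Blackboard and stops movement, then undoes the overlay and flag after a delay.
; Move issues AIMoveTo only while unfrozen.
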(event Custom|Freeze
  (bind (_blackboard _varoutput) (CallFunction|FUNCBBData "Frozen"))
  (bind _self self)
  (bind _rootcomponent (Variables|Transformation|GetRootComponent _self))
  (bind _returnvalue (Class|SceneComponent|GetNumChildrenComponents _rootcomponent))
  (if (not (Variables|Default|GetFrozen))
    (Variables|Default|SetFrozen true)
    (Development|PrintString (Utilities|String|ToString(Integer) _returnvalue))
    (for _index (range 0 _returnvalue)
      (bind _asstatic_mesh_component (Utilities|Casting|CastToStaticMeshComponent (Components|GetChildComponent (Variables|Transformation|GetRootComponent self) _index)))
      (Rendering|Material|SetOverlayMaterial _asstatic_mesh_component "/Game/GameContent/Materials/MAT_FreezeOverlay.MAT_FreezeOverlay" :!class /Script/Engine.MeshComponent))
    (AI|Components|Blackboard|SetValueasBool _blackboard _varoutput true)
    (Components|Movement|StopMovementImmediately (Variables|Character|GetCharacterMovement))
    (CallFunction|UnFreeze)))

(event Custom|UnFreeze
  (bind (_blackboard _varoutput) (CallFunction|FUNCBBData "Frozen"))
  (Utilities|FlowControl|Delay 3.0)
  (for _index (range 0 (Class|SceneComponent|GetNumChildrenComponents (Variables|Transformation|GetRootComponent self)))
    (bind _asstatic_mesh_component (Utilities|Casting|CastToStaticMeshComponent (Components|GetChildComponent (Variables|Transformation|GetRootComponent self) _index)))
    (Rendering|Material|SetOverlayMaterial _asstatic_mesh_component 0 :!class /Script/Engine.MeshComponent))
  (AI|Components|Blackboard|SetValueasBool _blackboard _varoutput false)
  (Variables|Default|SetFrozen false))

(event Custom|IsDead?
  (if (<= (Variables|Default|GetHealth) 0.0)
    (bind _returnvalue (Actor|GetActorOfClass "/Game/GameContent/Blueprints/Core/BP_EnemyManager.BP_EnemyManager_C"))
    (bind _output_get (Variables|/Game/GameContent/Blueprints/Core/BP_EnemyManager.BP_EnemyManager_C|SetEnemiesLeft _returnvalue (- (Variables|/Game/GameContent/Blueprints/Core/BP_EnemyManager.BP_EnemyManager_C|GetEnemiesLeft _returnvalue) 1)))
    (if (<= _output_get 0)
      (Default|ClearDoors _returnvalue))
    (Actor|DestroyActor)))

(event Custom|Move
  (params (Location :type Vector))
  (if (not (Variables|Default|GetFrozen))
    (AI|AIMoveTo self Location 0 1.4e+02 false)))

(event Game|Damage|EventAnyDamage
  (params (Damage :type Float%20%28single-precision%29) (DamageType :type Damage%20Type%20Object%20Reference) (InstigatedBy :type Controller%20Object%20Reference) (DamageCauser :type Actor%20Object%20Reference))
  (Variables|Default|SetHealth (- (Variables|Default|GetHealth) Damage))
  (CallFunction|IsDead?))

(fn ConstructionScript)

(fn FUNCBBData
  (params (VarName :type Name))
  (return (AI|GetBlackboard (AI|GetAIController self)) VarName))