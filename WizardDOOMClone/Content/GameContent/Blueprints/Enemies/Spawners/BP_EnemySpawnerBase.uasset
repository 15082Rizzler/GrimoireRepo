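; Base enemy spawner Blueprint that spawns one enemy for a specific room and wave.
; SpawnEnemy acts only when its MyRoom and MyWave match the current room and wave, then spawns EnemyToSpawn at its own location and rotation, adjusting for collisions but always spawning.
; Each successful spawn increments EnemiesLeft on the BP_EnemyManager found in the level, while a failed spawn prints an error.
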(event Custom|SpawnEnemy
  (bind _returnvalue (Transformation|GetActorTransform))
  (if (== (Variables|Default|GetMyRoom) (Variables|Default|GetCurrentRoom))
    (if (== (Variables|Default|GetMyWave) (Variables|Default|GetCurrentWave))
      (bind _returnvalue_2 (Game|SpawnActorfromClass (Variables|Default|GetEnemyToSpawn) (Math|Transform|MakeTransform (.location _returnvalue) (.rotation _returnvalue) "1.000000,1.000000,1.000000") "AdjustIfPossibleButAlwaysSpawn" "MultiplyWithRoot" 0 0))
      (Utilities|IsValid _returnvalue_2
        (:Is%20Valid
          (bind _returnvalue_3 (Actor|GetActorOfClass "/Game/GameContent/Blueprints/Core/BP_EnemyManager.BP_EnemyManager_C"))
          (Math|Integer|IncrementInt (Variables|/Game/GameContent/Blueprints/Core/BP_EnemyManager.BP_EnemyManager_C|GetEnemiesLeft _returnvalue_3)))
        (:Is%20Not%20Valid
          (Development|PrintString "Enemy failed to spawn!"))))))

(fn ConstructionScript)