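; Eye turret enemy Blueprint that fires projectiles through its Shoot event.
; After a short delay, Shoot spawns a BP_EnemyProjectileBase at the ShootPoint's location and rotation, unless the turret is Frozen.
; Either way, it then sets the CanShoot Blackboard key back to true.
; The construction script only calls its parent's.
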(event Custom|Shoot
  (bind (_blackboard _varoutput) (CallFunction|FUNCBBData "CanShoot"))
  (bind (_blackboard_2 _varoutput_2) (CallFunction|FUNCBBData "CanShoot"))
  (bind _shootpoint (Variables|Default|GetShootPoint))
  (Utilities|FlowControl|Delay 1.0)
  (if (Variables|Default|GetFrozen)
    (AI|Components|Blackboard|SetValueasBool _blackboard _varoutput true)
    (else
      (Game|SpawnActorfromClass "/Game/GameContent/Blueprints/Spells/EnemyProjectiles/BP_EnemyProjectileBase.BP_EnemyProjectileBase_C" (Math|Transform|MakeTransform (Transformation|GetWorldLocation _shootpoint) (Transformation|GetWorldRotation _shootpoint) "1.000000,1.000000,1.000000") "Undefined" "OverrideRootScale" 0 0)
      (AI|Components|Blackboard|SetValueasBool _blackboard_2 _varoutput_2 true))))

(fn ConstructionScript
  (|CallParentFunction))