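; BP_DamageBox is a short-lived hit volume that damages the player on overlap and destroys itself about a third of a second after BeginPlay.
; WhoSpawnedMe? stores the actor that spawned it.
; Overlapping a BP_RetaliateBarrier disables player damage and deals double damage back to that spawner.
; Each overlap branch passes through a DoOnce, so barrier retaliation and player damage fire at most once.
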(event OnComponentBeginOverlap(Box)
  (params (OverlappedComponent :type Primitive%20Component%20Object%20Reference) (OtherActor :type Actor%20Object%20Reference) (OtherComp :type Primitive%20Component%20Object%20Reference) (OtherBodyIndex :type Integer) (bFromSweep :type Boolean) (SweepResult :type Hit%20Result%20Structure%20%28by%20ref%29))
  (bind _asbp_retaliate_barrier (Utilities|Casting|CastToBP_RetaliateBarrier OtherActor)
    (:then
      (Utilities|IsValid _asbp_retaliate_barrier
        (:Is%20Valid
          (Utilities|FlowControl|DoOnce false
            (:Completed
              (Variables|Default|SetCan%20hurt%20player false)
              (Game|Damage|ApplyDamage (Variables|Default|GetActorWhoSpawnedMe) (* (Variables|Default|GetDamage) 2.0) 0 0))))))
    (:CastFailed
      (bind _asbp_player_character (Utilities|Casting|CastToBP_PlayerCharacter OtherActor))
      (Utilities|IsValid _asbp_player_character
        (:Is%20Valid
          (Utilities|FlowControl|DoOnce false
            (:Completed
              (if (Variables|Default|GetCan%20hurt%20player)
                (Game|Damage|ApplyDamage _asbp_player_character (Variables|Default|GetDamage) 0 0)))))))))

(event Custom|WhoSpawnedMe?
  (params (Actor :type Actor%20Object%20Reference))
  (Variables|Default|SetActorWhoSpawnedMe Actor))

(event EventBeginPlay
  (Utilities|FlowControl|Delay 0.334)
  (Actor|DestroyActor))

(fn ConstructionScript)