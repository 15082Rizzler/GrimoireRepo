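; BP_ProjectileParticleFollower is a standalone actor that plays a Niagara effect while tracking another actor, by its name a projectile.
; On BeginPlay it assigns its configured particle asset, then destroys itself after a fixed delay.
; FollowThis sets the tracked actor, whose location and rotation it copies each Tick while valid, without attachment.
; StopParticleLooping deactivates the effect separately from the actor's destruction.
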(event Custom|FollowThis
  (params (ActorInput :type Actor%20Object%20Reference))
  (Variables|Default|SetFollowedActor ActorInput))

(event Custom|StopParticleLooping
  (Components|Activation|Deactivate (Variables|Default|GetNiagara)))

(event EventBeginPlay
  (Class|NiagaraComponent|SetAsset (Variables|Default|GetNiagara) (Variables|Default|GetParticleAsset) true)
  (Utilities|FlowControl|Delay 12.0)
  (Actor|DestroyActor))

(event EventTick
  (params (DeltaSeconds :type Float%20%28single-precision%29))
  (bind _followedactor (Variables|Default|GetFollowedActor))
  (Utilities|IsValid (Variables|Default|GetFollowedActor)
    (:Is%20Valid
      (Transformation|SetActorLocationAndRotation (Transformation|GetActorLocation _followedactor) (Transformation|GetActorRotation _followedactor)))))

(fn ConstructionScript)