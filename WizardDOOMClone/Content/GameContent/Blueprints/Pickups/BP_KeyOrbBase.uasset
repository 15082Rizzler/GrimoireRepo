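; BP_KeyOrbBase is a key orb pickup that grants the player a blue, red or green key.
; On actor overlap it casts to BP_PlayerCharacter, calls the character's key function matching its KeyType, then destroys itself.
; An unmatched KeyType prints a warning with the orb's display name and leaves the orb in place.
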(event Collision|EventActorBeginOverlap
  (params (OtherActor :type Actor%20Object%20Reference))
  (bind _asbp_player_character (Utilities|Casting|CastToBP_PlayerCharacter OtherActor))
  (switch int (Variables|Default|GetKeyType)
    (:Default
      (Development|PrintString (Utilities|String|Append "No KeyType Inputted!" " || " (Utilities|GetDisplayName self))))
    (:0
      (Default|GetBlueKey _asbp_player_character)
      (Actor|DestroyActor :!label _label))
    (:1
      (Default|GetRedKey _asbp_player_character)
      (goto _label))
    (:2
      (Default|GetGreenKey _asbp_player_character)
      (goto _label))))

(fn ConstructionScript)