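; Base spell pickup actor that grants the player one of eight spells when touched.
; On begin overlap it casts the other actor to BP_PlayerCharacter and switches on SpellType to call the matching Get function, covering attack and movement spells such as Fireball and Wind Dash.
; Each case then destroys the pickup, while overlaps from any other actor are ignored.
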(event Collision|EventActorBeginOverlap
  (params (OtherActor :type Actor%20Object%20Reference))
  (bind _asbp_player_character (Utilities|Casting|CastToBP_PlayerCharacter OtherActor))
  (switch int (Variables|Default|GetSpellType)
    (:0
      (Default|GetMagicMissile _asbp_player_character)
      (Actor|DestroyActor))
    (:1
      (Default|GetWindDash _asbp_player_character)
      (Actor|DestroyActor))
    (:2
      (Default|GetLightningJump _asbp_player_character)
      (Actor|DestroyActor))
    (:3
      (Default|GetRetaliate _asbp_player_character)
      (Actor|DestroyActor))
    (:4
      (Default|GetFireball _asbp_player_character)
      (Actor|DestroyActor))
    (:5
      (Default|GetLightningBolt _asbp_player_character)
      (Actor|DestroyActor))
    (:6
      (Default|GetFreezingIcicle _asbp_player_character)
      (Actor|DestroyActor))
    (:7
      (Default|GetRockWall _asbp_player_character)
      (Actor|DestroyActor))))

(fn ConstructionScript)