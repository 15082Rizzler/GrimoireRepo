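; A debug trigger Blueprint that tests enemy wave spawning when its box component is overlapped.
; Each overlap switches on WaveNumber: for waves one to three it finds BP_EnemyManager, calls ChangeWave with the current number, then increments it and prints a message.
; Zero silently becomes wave one, and any value past the last wave resets to one with a printed notice.
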(event OnComponentBeginOverlap(Box)
  (params (OverlappedComponent :type Primitive%20Component%20Object%20Reference) (OtherActor :type Actor%20Object%20Reference) (OtherComp :type Primitive%20Component%20Object%20Reference) (OtherBodyIndex :type Integer) (bFromSweep :type Boolean) (SweepResult :type Hit%20Result%20Structure%20%28by%20ref%29))
  (switch int (Variables|Default|GetWaveNumber)
    (:Default
      (Variables|Default|SetWaveNumber 1)
      (Development|PrintString "Reset waves!"))
    (:0
      (Variables|Default|SetWaveNumber 1))
    (:1
      (bind _returnvalue (Actor|GetActorOfClass "/Game/GameContent/Blueprints/Core/BP_EnemyManager.BP_EnemyManager_C"))
      (Default|ChangeWave _returnvalue (Variables|Default|GetWaveNumber))
      (Math|Integer|IncrementInt (Variables|Default|GetWaveNumber)
        (:%20%20
          (Development|PrintString "Spawning wave 1!"))))
    (:2
      (bind _returnvalue_2 (Actor|GetActorOfClass "/Game/GameContent/Blueprints/Core/BP_EnemyManager.BP_EnemyManager_C"))
      (Default|ChangeWave _returnvalue_2 (Variables|Default|GetWaveNumber))
      (Math|Integer|IncrementInt (Variables|Default|GetWaveNumber)
        (:%20%20
          (Development|PrintString "Spawning wave 2!"))))
    (:3
      (bind _returnvalue_3 (Actor|GetActorOfClass "/Game/GameContent/Blueprints/Core/BP_EnemyManager.BP_EnemyManager_C"))
      (Default|ChangeWave _returnvalue_3 (Variables|Default|GetWaveNumber))
      (Math|Integer|IncrementInt (Variables|Default|GetWaveNumber)
        (:%20%20
          (Development|PrintString "Spawning wave 3!"))))))

(fn ConstructionScript)