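; Enemy manager that drives wave spawning and room tracking for arena encounters.
; ChangeWave stores the wave number and triggers every spawner of the matching class (waves 1 to 3), passing it the wave.
; ChangeRoom pushes the current room number to all three spawner classes without spawning.
; ClearDoors opens every arena door, with all targets found through GetAllActorsOfClass lookups.
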(event Custom|ChangeWave
  (params (WaveNumber :type Integer))
  (bind _output_get (Variables|Default|SetCurrentWave WaveNumber))
  (CallFunction|FUNCEvaluateWave _output_get))

(event Custom|ChangeRoom
  (params (RoomNumber :type Integer))
  (bind _output_get (Variables|Default|SetCurrentRoom RoomNumber))
  (CallFunction|FUNCEvaluateRoom _output_get))

(event Custom|ClearDoors
  (bind _outactors (Actor|GetAllActorsOfClass "/Game/GameContent/Blueprints/LevelMechanics/BP_ArenaDoor.BP_ArenaDoor_C"))
  (for _array_element _outactors
    (Default|OpenDoor _array_element)))

(fn ConstructionScript)

(fn FUNCEvaluateWave
  (params (WaveNumber :type Integer))
  (switch int WaveNumber
    (:Default
      (Development|PrintString "Invalid wave number!" true true "(R=1.000000,G=0.000000,B=0.000000,A=1.000000)"))
    (:0
      (Development|PrintString "Accidentally set the wave to 0. Start at 1 dummy!" true true "(R=1.000000,G=0.000000,B=0.000000,A=1.000000)"))
    (:1
      (bind _outactors (Actor|GetAllActorsOfClass "/Game/GameContent/Blueprints/Enemies/Spawners/BP_Wave1Spawner.BP_Wave1Spawner_C"))
      (for _array_element _outactors
        (Variables|/Game/GameContent/Blueprints/Enemies/Spawners/BP_EnemySpawnerBase.BP_EnemySpawnerBase_C|SetCurrentWave _array_element (Variables|Default|GetCurrentWave))
        (Default|SpawnEnemy _array_element)))
    (:2
      (bind _outactors_2 (Actor|GetAllActorsOfClass "/Game/GameContent/Blueprints/Enemies/Spawners/BP_Wave2Spawner.BP_Wave2Spawner_C"))
      (for _array_element_2 _outactors_2
        (Variables|/Game/GameContent/Blueprints/Enemies/Spawners/BP_EnemySpawnerBase.BP_EnemySpawnerBase_C|SetCurrentWave _array_element_2 (Variables|Default|GetCurrentWave))
        (Default|SpawnEnemy _array_element_2)))
    (:3
      (bind _outactors_3 (Actor|GetAllActorsOfClass "/Game/GameContent/Blueprints/Enemies/Spawners/BP_Wave3Spawner.BP_Wave3Spawner_C"))
      (for _array_element_3 _outactors_3
        (Variables|/Game/GameContent/Blueprints/Enemies/Spawners/BP_EnemySpawnerBase.BP_EnemySpawnerBase_C|SetCurrentWave _array_element_3 (Variables|Default|GetCurrentWave))
        (Default|SpawnEnemy _array_element_3)))))

(fn FUNCEvaluateRoom
  (params (RoomNumber :type Integer))
  (Utilities|FlowControl|Sequence
    (:then_0
      (bind _outactors (Actor|GetAllActorsOfClass "/Game/GameContent/Blueprints/Enemies/Spawners/BP_Wave1Spawner.BP_Wave1Spawner_C"))
      (for _array_element _outactors
        (Variables|/Game/GameContent/Blueprints/Enemies/Spawners/BP_EnemySpawnerBase.BP_EnemySpawnerBase_C|SetCurrentRoom _array_element (Variables|Default|GetCurrentRoom))))
    (:then_1
      (bind _outactors_2 (Actor|GetAllActorsOfClass "/Game/GameContent/Blueprints/Enemies/Spawners/BP_Wave2Spawner.BP_Wave2Spawner_C"))
      (for _array_element_2 _outactors_2
        (Variables|/Game/GameContent/Blueprints/Enemies/Spawners/BP_EnemySpawnerBase.BP_EnemySpawnerBase_C|SetCurrentRoom _array_element_2 (Variables|Default|GetCurrentRoom))))
    (:then_2
      (bind _outactors_3 (Actor|GetAllActorsOfClass "/Game/GameContent/Blueprints/Enemies/Spawners/BP_Wave3Spawner.BP_Wave3Spawner_C"))
      (for _array_element_3 _outactors_3
        (Variables|/Game/GameContent/Blueprints/Enemies/Spawners/BP_EnemySpawnerBase.BP_EnemySpawnerBase_C|SetCurrentRoom _array_element_3 (Variables|Default|GetCurrentRoom))))))