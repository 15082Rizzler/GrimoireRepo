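; BP_RoomChanger is a box trigger that starts an arena encounter when the player character enters it.
; On the first player overlap it passes its room and wave numbers to BP_EnemyManager, then closes every BP_ArenaDoor in the level.
; A DoOnce gate prevents retriggering until ResetRC re-arms it.
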(event OnComponentBeginOverlap(Box)
  (params (OverlappedComponent :type Primitive%20Component%20Object%20Reference) (OtherActor :type Actor%20Object%20Reference) (OtherComp :type Primitive%20Component%20Object%20Reference) (OtherBodyIndex :type Integer) (bFromSweep :type Boolean) (SweepResult :type Hit%20Result%20Structure%20%28by%20ref%29))
  (Utilities|Casting|CastToBP_PlayerCharacter OtherActor)
  (Utilities|FlowControl|DoOnce false
    (:Completed
      (bind _returnvalue (Actor|GetActorOfClass "/Game/GameContent/Blueprints/Core/BP_EnemyManager.BP_EnemyManager_C"))
      (Default|ChangeRoom _returnvalue (Variables|Default|GetRoomNumber))
      (Default|ChangeWave _returnvalue (Variables|Default|GetWaveNumber))
      (bind _outactors (Actor|GetAllActorsOfClass "/Game/GameContent/Blueprints/LevelMechanics/BP_ArenaDoor.BP_ArenaDoor_C"))
      (for _array_element _outactors
        (Default|CloseDoor _array_element)))))

(event Custom|ResetRC
  (Utilities|FlowControl|DoOnce false) ; enters at Reset
)

(fn ConstructionScript)