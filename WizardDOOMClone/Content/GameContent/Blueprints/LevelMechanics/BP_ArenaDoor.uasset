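; BP_ArenaDoor is a level mechanic door that blocks or frees passage in an arena by appearing and disappearing.
; It starts open, calling OpenDoor on BeginPlay to hide the Scene component and its children and disable the Cube's collision.
; CloseDoor restores visibility and query-and-physics collision, with no animation or movement, and nothing in this Blueprint calls it.
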(event Custom|OpenDoor
  (Rendering|SetVisibility (Variables|Default|GetScene) false true)
  (Collision|SetCollisionEnabled (Variables|Default|GetCube) "NoCollision"))

(event Custom|CloseDoor
  (Rendering|SetVisibility (Variables|Default|GetScene) true true)
  (Collision|SetCollisionEnabled (Variables|Default|GetCube) "QueryAndPhysics"))

(event EventBeginPlay
  (CallFunction|OpenDoor))

(fn ConstructionScript)