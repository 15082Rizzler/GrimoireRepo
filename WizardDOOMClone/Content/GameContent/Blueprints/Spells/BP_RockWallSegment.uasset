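; BP_RockWallSegment is a spell actor that forms a short-lived segment of rock wall from cube components.
; On BeginPlay it loops over its centre, left, centre-left and right cubes, randomizing each Z scale while keeping X and Y for an uneven height.
; The centre cube appears twice in that loop, so it is randomized twice.
; After a fixed five-second delay the segment destroys itself.
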(event EventBeginPlay
  (for _array_element (Utilities|Array|MakeArray (Variables|Default|GetCubeCentre) (Variables|Default|GetCubeLeft) (Variables|Default|GetCubeCentreLeft) (Variables|Default|GetCubeRight) (Variables|Default|GetCubeCentre))
    (Transformation|SetWorldScale3D _array_element (Math|Vector|MakeVector (.x (Transformation|GetWorldScale _array_element)) (.y (Transformation|GetWorldScale _array_element)) (Math|Random|RandomFloatinRange 5.0 7.0))))
  (Utilities|FlowControl|Delay 5.0)
  (Actor|DestroyActor))

(fn ConstructionScript)