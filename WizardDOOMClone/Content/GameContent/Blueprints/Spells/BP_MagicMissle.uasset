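; BP_MagicMissle is a magic missile spell projectile that damages enemies on hit.
; On BeginPlay it spawns a separate particle follower actor to track it, then destroys itself after a fixed delay.
; Hitting a BP_EnemyBase applies damage and a velocity-scaled impulse to physics-simulating components.
; Any hit stops the follower's particle looping and destroys the missile, but the timeout path skips that stop call.
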(event EventBeginPlay
  (bind _returnvalue (Game|SpawnActorfromClass "/Game/GameContent/Blueprints/Particles/BP_ProjectileParticleFollower.BP_ProjectileParticleFollower_C" (Math|Transform|MakeTransform (Transformation|GetActorLocation) "0, 0, 0" "1.000000,1.000000,1.000000") "Undefined" "MultiplyWithRoot" 0 0))
  (Variables|Default|SetMyParticles _returnvalue)
  (Default|FollowThis _returnvalue self)
  (Utilities|FlowControl|Delay 12.0)
  (Actor|DestroyActor))

(event Collision|EventHit
  (params (MyComp :type Primitive%20Component%20Object%20Reference) (Other :type Actor%20Object%20Reference) (OtherComp :type Primitive%20Component%20Object%20Reference) (bSelfMoved :type Boolean) (HitLocation :type Vector :default "0, 0, 0") (HitNormal :type Vector :default "0, 0, 0") (NormalImpulse :type Vector :default "0, 0, 0") (Hit :type Hit%20Result%20Structure%20%28by%20ref%29))
  (Utilities|Casting|CastToBP_EnemyBase Other
    (:then
      (if (Physics|IsSimulatingPhysics OtherComp "None")
        (Physics|AddImpulseatLocation OtherComp (* (Transformation|GetVelocity) 1e+02) (Transformation|GetActorLocation) "None"))
      (Game|Damage|ApplyDamage Other 2e+01 0 0)
      (Default|StopParticleLooping (Variables|Default|GetMyParticles))
      (Actor|DestroyActor))
    (:CastFailed
      (Default|StopParticleLooping (Variables|Default|GetMyParticles))
      (Actor|DestroyActor))))

(fn ConstructionScript)