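; Base enemy projectile actor that damages what it hits and destroys itself after 12 seconds if still alive.
; On hit, player characters and enemies alike take damage, and a simulating hit component also gets an impulse scaled from the projectile's velocity.
; The projectile is destroyed after any hit, with no damage or impulse applied to other actor types.
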(event EventBeginPlay
  (Utilities|FlowControl|Delay 12.0)
  (Actor|DestroyActor))

(event Collision|EventHit
  (params (MyComp :type Primitive%20Component%20Object%20Reference) (Other :type Actor%20Object%20Reference) (OtherComp :type Primitive%20Component%20Object%20Reference) (bSelfMoved :type Boolean) (HitLocation :type Vector :default "0, 0, 0") (HitNormal :type Vector :default "0, 0, 0") (NormalImpulse :type Vector :default "0, 0, 0") (Hit :type Hit%20Result%20Structure%20%28by%20ref%29))
  (Utilities|Casting|CastToBP_PlayerCharacter Other
    (:then
      (if (Physics|IsSimulatingPhysics OtherComp "None") :!label _label
        (Physics|AddImpulseatLocation OtherComp (* (Transformation|GetVelocity) 1e+02) (Transformation|GetActorLocation) "None"))
      (Game|Damage|ApplyDamage Other (Variables|Default|GetDamage) 0 0)
      (Actor|DestroyActor))
    (:CastFailed
      (Utilities|Casting|CastToBP_EnemyBase Other
        (:then
          (goto _label))
        (:CastFailed
          (Actor|DestroyActor))))))

(fn ConstructionScript)