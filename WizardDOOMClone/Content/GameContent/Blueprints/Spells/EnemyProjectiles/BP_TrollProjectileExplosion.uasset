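; BP_TrollProjectileExplosion is a short-lived explosion actor for the troll enemy projectile that deals area damage when spawned.
; On BeginPlay it runs a multi sphere object trace at its root location, ignoring all actors of one class, and applies flat damage for each hit.
; It then destroys itself after a delay.
; The trace has debug drawing on, and hits are not de-duplicated per actor.
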(event EventBeginPlay
  (bind _defaultsceneroot (Variables|Default|GetDefaultSceneRoot))
  (bind _returnvalue (Transformation|GetWorldLocation _defaultsceneroot))
  (bind _outactors (Actor|GetAllActorsOfClass 0))
  (Variables|Default|SetActors%20to%20Ignore _outactors)
  (bind _outhits (Collision|MultiSphereTraceForObjects _returnvalue _returnvalue 2.2e+02 (Variables|Default|GetObject%20Types) false (Variables|Default|GetActors%20to%20Ignore) "ForDuration"))
  (for _array_element _outhits
    (Game|Damage|ApplyDamage (.HitActor (Collision|BreakHitResult _array_element)) 2e+01 0 0))
  (Utilities|FlowControl|Delay 5.0)
  (Actor|DestroyActor))

(fn ConstructionScript)