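; Fireball explosion spell actor that deals one burst of area damage where it spawns.
; On BeginPlay it plays an explosion sound and runs a zero-length multi sphere trace at its root, filtered by an object type list.
; Each hit applies flat damage with no falloff or per-actor deduplication, and the trace's debug drawing is left on.
; The actor destroys itself after a short delay.
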(event EventBeginPlay
  (bind _defaultsceneroot (Variables|Default|GetDefaultSceneRoot))
  (bind _returnvalue (Transformation|GetWorldLocation _defaultsceneroot))
  (Audio|PlaySoundatLocation "/Game/GameContent/Sounds/explosion-fx-343683.explosion-fx-343683" (Transformation|GetActorLocation) "0, 0, 0" 1.0 1.0 0.0 0 0 0 0)
  (bind _outhits (Collision|MultiSphereTraceForObjects _returnvalue _returnvalue 2.2e+02 (Variables|Default|GetObject%20Types) false 0 "ForDuration"))
  (for _array_element _outhits
    (Game|Damage|ApplyDamage (.HitActor (Collision|BreakHitResult _array_element)) 5e+01 0 0))
  (Utilities|FlowControl|Delay 5.0)
  (Actor|DestroyActor))

(fn ConstructionScript)