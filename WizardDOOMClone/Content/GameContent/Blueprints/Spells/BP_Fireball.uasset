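; Fireball spell projectile that explodes on impact and damages enemies.
; On hit it spawns BP_FireballExplosion at its location and destroys itself, whatever it struck.
; Hits on BP_EnemyBase actors also apply fixed damage and push physics-simulating components with a velocity-scaled impulse.
; A timer started on BeginPlay destroys it without an explosion if it hits nothing.
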(event EventBeginPlay
  (Utilities|FlowControl|Delay 12.0)
  (Actor|DestroyActor))

(event Collision|EventHit
  (params (MyComp :type Primitive%20Component%20Object%20Reference) (Other :type Actor%20Object%20Reference) (OtherComp :type Primitive%20Component%20Object%20Reference) (bSelfMoved :type Boolean) (HitLocation :type Vector :default "0, 0, 0") (HitNormal :type Vector :default "0, 0, 0") (NormalImpulse :type Vector :default "0, 0, 0") (Hit :type Hit%20Result%20Structure%20%28by%20ref%29))
  (bind _returnvalue (Transformation|GetActorLocation))
  (Utilities|Casting|CastToBP_EnemyBase Other
    (:then
      (if (Physics|IsSimulatingPhysics OtherComp "None")
        (Physics|AddImpulseatLocation OtherComp (* (Transformation|GetVelocity) 1e+02) _returnvalue "None"))
      (Game|SpawnActorfromClass "/Game/GameContent/Blueprints/Spells/BP_FireballExplosion.BP_FireballExplosion_C" (Math|Transform|MakeTransform _returnvalue "0, 0, 0" "1.000000,1.000000,1.000000") "Undefined" "MultiplyWithRoot" 0 0)
      (Game|Damage|ApplyDamage Other 5e+01 0 0)
      (Actor|DestroyActor))
    (:CastFailed
      (Game|SpawnActorfromClass "/Game/GameContent/Blueprints/Spells/BP_FireballExplosion.BP_FireballExplosion_C" (Math|Transform|MakeTransform (Transformation|GetActorLocation) "0, 0, 0" "1.000000,1.000000,1.000000") "Undefined" "MultiplyWithRoot" 0 0)
      (Actor|DestroyActor))))

(fn ConstructionScript)