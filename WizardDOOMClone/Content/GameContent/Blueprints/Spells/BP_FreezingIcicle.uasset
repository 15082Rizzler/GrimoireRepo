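; BP_FreezingIcicle is a spell projectile that damages and freezes enemies it hits.
; On hit, a BP_EnemyBase takes damage and has Freeze called, and its hit component receives a velocity-scaled impulse if simulating physics.
; Any hit plays an impact sound and destroys the icicle, which otherwise expires after a fixed lifetime.
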(event EventBeginPlay
  (Utilities|FlowControl|Delay 12.0)
  (Actor|DestroyActor))

(event Collision|EventHit
  (params (MyComp :type Primitive%20Component%20Object%20Reference) (Other :type Actor%20Object%20Reference) (OtherComp :type Primitive%20Component%20Object%20Reference) (bSelfMoved :type Boolean) (HitLocation :type Vector :default "0, 0, 0") (HitNormal :type Vector :default "0, 0, 0") (NormalImpulse :type Vector :default "0, 0, 0") (Hit :type Hit%20Result%20Structure%20%28by%20ref%29))
  (bind _asbp_enemy_base (Utilities|Casting|CastToBP_EnemyBase Other)
    (:then
      (if (Physics|IsSimulatingPhysics OtherComp "None")
        (Physics|AddImpulseatLocation OtherComp (* (Transformation|GetVelocity) 1e+02) (Transformation|GetActorLocation) "None"))
      (Game|Damage|ApplyDamage Other 1e+01 0 0)
      (Audio|PlaySoundatLocation "/Game/GameContent/Sounds/IcicleImpactSFX.IcicleImpactSFX" (Transformation|GetActorLocation) "0, 0, 0" 1.0 1.0 0.0 0 0 0 0)
      (Utilities|IsValid _asbp_enemy_base
        (:Is%20Valid
          (Default|Freeze _asbp_enemy_base))
        (:Is%20Not%20Valid
          _))
      (Actor|DestroyActor))
    (:CastFailed
      (Audio|PlaySoundatLocation "/Game/GameContent/Sounds/IcicleImpactSFX.IcicleImpactSFX" (Transformation|GetActorLocation) "0, 0, 0" 1.0 1.0 0.0 0 0 0 0)
      (Actor|DestroyActor))))

(fn ConstructionScript)